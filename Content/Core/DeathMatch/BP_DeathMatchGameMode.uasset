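; Game mode for a two-team Aliens vs Humans ship deathmatch, handling team assignment, spawning, respawns and scoring.
; PostLogin fills teams by a player counter, and FindPlayerStart spawns a PlayerStart at the player's team location.
; On death, the opposing team scores and the same pawn teleports to its team spawn with health and shield restored.
; Tick polls both scores against WinScore and sends a one-time game-over event to player controllers.
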(event Custom|GameOver
  (CallFunction|WinCondition))

(event Custom|Respawn
  (params (Pawn :type BP%20Ship%20Object%20Reference))
  (CallFunction|RespawnEventHandler Pawn))

(event EventTick
  (params (DeltaSeconds :type Float%20%28single-precision%29))
  (CallFunction|GameOver))

(event EventBeginPlay
  (EventDispatchers|BindEventtoOnPlayerDied (delegate Custom|Respawn)))

(event EventPostLogin
  (params (NewPlayer :type Player%20Controller%20Object%20Reference))
  (CallFunction|AssignTeamforNewPlayer NewPlayer))

(fn ConstructionScript)

(fn AssignTeamforNewPlayer
  (params (NewPlayer :type Player%20Controller%20Object%20Reference))
  (bind _asbp_death_match_player_controller (Utilities|Casting|CastToBP_DeathMatchPlayerController NewPlayer))
  (bind _currentteam (Variables|Teams|GetCurrentTeam))
  (bind _playersbyteam (Variables|Teams|GetPlayersByTeam))
  (bind _value (Utilities|Map|Find _playersbyteam _currentteam))
  (bind _playerstate (Variables|/Script/Engine.Controller|GetPlayerState _asbp_death_match_player_controller))
  (bind _asbp_death_match_player_state (Utilities|Casting|CastToBP_DeathMatchPlayerState _playerstate))
  (if (== (Variables|Teams|GetTeamIndex) (Variables|Teams|GetPlayersNumber))
    (Variables|/Game/Core/DeathMatch/BP_DeathMatchPlayerState.BP_DeathMatchPlayerState_C|SetTeamIndex _asbp_death_match_player_state (Variables|Teams|GetCurrentTeam))
    (Utilities|Array|Add (.players _value) _asbp_death_match_player_state)
    (Variables|Teams|SetTeamIndex 1)
    (Math|Integer|IncrementInt (Variables|Teams|GetCurrentTeam))
    (else
      (Utilities|Map|Add (Variables|Teams|GetPlayersByTeam) (Variables|Teams|GetCurrentTeam) (Utilities|Struct|MakeS_PlayersByTeam))
      (Variables|/Game/Core/DeathMatch/BP_DeathMatchPlayerState.BP_DeathMatchPlayerState_C|SetTeamIndex _asbp_death_match_player_state (Variables|Teams|GetCurrentTeam))
      (Utilities|Array|Add (.players _value) _asbp_death_match_player_state)
      (Math|Integer|IncrementInt (Variables|Teams|GetTeamIndex)))))

(fn GetTeamSpawnPoint
  (params (Team%20Number :type Integer))
  (switch int Team%20Number
    (:1
      (return (Variables|SpawnLocations|GetFirstTeamSpawnLocation)))
    (:2
      (return (Variables|SpawnLocations|GetSecondTeamSpawnLocation)))))

(fn FindPlayerStart
  (params (Player :type Controller%20Object%20Reference) (IncomingName :type String))
  (bind _asbp_death_match_player_state (Utilities|Casting|CastToBP_DeathMatchPlayerState (Variables|/Script/Engine.Controller|GetPlayerState Player)))
  (bind _spawn_location (CallFunction|GetTeamSpawnPoint (Variables|/Game/Core/DeathMatch/BP_DeathMatchPlayerState.BP_DeathMatchPlayerState_C|GetTeamIndex _asbp_death_match_player_state)))
  (bind _returnvalue (Game|SpawnActorfromClass "/Script/Engine.PlayerStart" (Math|Transform|MakeTransform _spawn_location "0, 0, 0" "1.000000,1.000000,1.000000") "AlwaysSpawn" 0 0))
  (return _returnvalue))

(fn ResetPlayerHP
  (params (Player%20Ship :type BP%20Ship%20Object%20Reference))
  (bind _healthcomponent (Variables|/Script/ZeroGoki.SpaceShip|GetHealthComponent Player%20Ship))
  (Class|HealthComponent|SetCurrentHealth _healthcomponent (Class|HealthComponent|GetMaxHealth _healthcomponent))
  (Class|HealthComponent|SetCurrentShield _healthcomponent (Class|HealthComponent|GetMaxShield _healthcomponent)))

(fn GetScorebyTeam
  (params (Team%20Index :type Integer))
  (for _array_element (.players (.Value (Utilities|Map|Find (Variables|Teams|GetPlayersByTeam) Team%20Index)))
    (LocalVariables|SetTeamScore (+ (Variables|/Script/ZeroGoki.ZeroGokiPlayerState|GetKills _array_element) (LocalVariables|GetTeamScore))))
  (return (LocalVariables|GetTeamScore)))

(fn AddTeamPoints
  (params (Opponents%20Team :type Integer))
  (switch int Opponents%20Team
    (:1
      (Variables|Score|SetAliensScore (+ (select (== Opponents%20Team 1) (Variables|Score|GetAliensScore) (Variables|Score|GetHumansScore)) 1)))
    (:2
      (Variables|Score|SetHumansScore (+ (select (== Opponents%20Team 1) (Variables|Score|GetAliensScore) (Variables|Score|GetHumansScore)) 1)))))

(fn WinCondition
  (bind _winscore (Variables|Score|GetWinScore))
  (bind _aliensscore (Variables|Score|GetAliensScore))
  (bind _returnvalue (== _winscore _aliensscore))
  (if (not (Variables|Default|GetbIsGameOver))
    (if _returnvalue
      (Variables|Default|SetbIsGameOver true :!label _label)
      (for _array_element (Variables|/Script/Engine.GameStateBase|GetPlayerArray (Game|GetGameState))
        (bind _asbp_death_match_player_controller (Utilities|Casting|CastToBP_DeathMatchPlayerController (Game|GetPlayerController _array_element)))
        (Default|GameOverEvent _asbp_death_match_player_controller (select _returnvalue 2 1)))
      (elif (== (Variables|Score|GetHumansScore) (Variables|Score|GetWinScore))
        (goto _label)))))

(fn RespawnEventHandler
  (params (Pawn :type BP%20Ship%20Object%20Reference))
  (bind _asbp_death_match_player_state (Utilities|Casting|CastToBP_DeathMatchPlayerState (Variables|/Script/Engine.Pawn|GetPlayerState Pawn)))
  (CallFunction|AddTeamPoints (Variables|/Script/ZeroGoki.ZeroGokiPlayerState|GetTeamIndex _asbp_death_match_player_state))
  (bind _spawn_location (CallFunction|GetTeamSpawnPoint (Variables|/Script/ZeroGoki.ZeroGokiPlayerState|GetTeamIndex _asbp_death_match_player_state)))
  (Transformation|SetActorLocation Pawn _spawn_location false true)
  (CallFunction|ResetPlayerHP Pawn))

(fn SetPlayersGameOverWidget
  (params (Game%20Over%20Widget :type WBP%20Game%20Over%20Object%20Reference)))