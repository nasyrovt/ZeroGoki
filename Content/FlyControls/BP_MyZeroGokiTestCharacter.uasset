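; Test player Character that flies as a spaceship, removing its default mesh and showing the main HUD at BeginPlay.
; Axis inputs steer controller yaw and pitch and drive movement along the control rotation, with a lerped roll banking the ship on turns.
; Actions toggle first/third-person view through spring arm length and open the pause menu widget.
; Every capsule hit subtracts fixed health and prints the result.
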(event OnComponentHit(CapsuleComponent)
  (params (HitComponent :type Primitive%20Component%20Object%20Reference) (OtherActor :type Actor%20Object%20Reference) (OtherComp :type Primitive%20Component%20Object%20Reference) (NormalImpulse :type Vector :default "0, 0, 0") (Hit :type Hit%20Result%20Structure%20%28by%20ref%29))
  ;[1 1 1] Take damage if spaceship hit something
  (Class|ZeroGokiTestCharacter|SetCurrentHealth (- (Class|ZeroGokiTestCharacter|GetCurrentHealth) 1e+01))
  (Development|PrintString (Utilities|String|ToString(Float) (Class|ZeroGokiTestCharacter|GetCurrentHealth))))

(event EventBeginPlay
  (Utilities|FlowControl|Sequence
    (:then_0
      (Components|DestroyComponent (Variables|Character|GetMesh)))
    (:then_1
      (CallFunction|AddUItoViewport))))

(event EventDestroyed
  (Development|PrintString "Character Destroyed"))

(event Input|ActionEvents|InputActionFPS/TPSCameraView
  (params (Key :type Key%20Structure :default "None"))
  (:Pressed
    (if (Variables|Default|GetbIsInFPSMode)
      (Variables|/Script/Engine.SpringArmComponent|SetTargetArmLength (Variables|Default|GetSpringArm) 5.1e+02)
      (Variables|Default|SetbIsInFPSMode false)
      (else
        (Variables|/Script/Engine.SpringArmComponent|SetTargetArmLength (Variables|Default|GetSpringArm) 2e+01)
        (Variables|Default|SetbIsInFPSMode true)))))

(event Input|ActionEvents|InputActionMenu
  (params (Key :type Key%20Structure :default "None"))
  (:Pressed
    (bind _returnvalue (UserInterface|CreateWidget "/Game/Widget/Pause_Menu.Pause_Menu_C"))
    (UserInterface|Viewport|AddtoViewport _returnvalue 0)))

(event Input|AxisEvents|InputAxisMoveForward/Backward
  (params (AxisValue :type Float%20%28single-precision%29))
  (Pawn|Input|AddMovementInput (Math|Vector|GetForwardVector (Pawn|GetControlRotation :!class /Script/Engine.Pawn)) (* AxisValue (Variables|Default|GetMovement%20Speed)) false))

(event Input|AxisEvents|InputAxisMoveUp
  (params (AxisValue :type Float%20%28single-precision%29))
  (Pawn|Input|AddControllerPitchInput AxisValue))

(event Input|AxisEvents|InputAxisMoveRight/Left
  (params (AxisValue :type Float%20%28single-precision%29))
  (bind _spaceship (Variables|Default|GetSpaceship))
  (Pawn|Input|AddControllerYawInput (* AxisValue (Variables|Default|GetTurnSpeed)))
  (Transformation|SetRelativeRotation _spaceship (Math|Rotator|MakeRotator (Math|Float|Clamp(Float) (Math|Float|Lerp (.roll (Variables|/Script/Engine.SceneComponent|GetRelativeRotation _spaceship)) (* AxisValue (Variables|Default|GetRoll%20Amount)) 0.09) -1e+03 1e+03) 0.0 0.0) false false))

(fn ConstructionScript)

(fn AddUItoViewport
  (bind _returnvalue (UserInterface|CreateWidget "/Game/Widget/UI_Main.UI_Main_C"))
  (UserInterface|Viewport|AddtoViewport _returnvalue 0))