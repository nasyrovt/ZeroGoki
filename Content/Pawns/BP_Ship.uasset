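; BP_Ship is a player ship pawn for a deathmatch game mode, handling death detection and respawning.
; Each Tick polls its HealthComponent and, while health is at or below zero, reports the ship to BP_DeathMatchGameMode through CallOnPlayerDied.
; A separate RespawnPlayer function caches the deathmatch player controller, destroys the ship, then has the game mode restart that player.
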(event EventTick
  (params (DeltaSeconds :type Float%20%28single-precision%29))
  (if (<= (Class|HealthComponent|GetCurrentHealth (Variables|Default|GetHealthComponent)) 0.0)
    (bind _asbp_death_match_game_mode (Utilities|Casting|CastToBP_DeathMatchGameMode (Game|GetGameMode)))
    (Default|CallOnPlayerDied _asbp_death_match_game_mode self)))

(fn ConstructionScript)

(fn RespawnPlayer
  (LocalVariables|SetControllerRef (.AsBP%20Death%20Match%20Player%20Controller (Utilities|Casting|CastToBP_DeathMatchPlayerController (Pawn|GetController))))
  (Actor|DestroyActor)
  (bind _asbp_death_match_game_mode (Utilities|Casting|CastToBP_DeathMatchGameMode (Game|GetGameMode)))
  (Class|GameModeBase|RestartPlayer _asbp_death_match_game_mode (LocalVariables|GetControllerRef)))